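; Base game mode for a bomber-tag style match that tracks connected players and runs rounds until one player remains.
; StartGame refuses a single player, otherwise resets winner state and gives a five-second head start.
; It then repeatedly clears current bombers and picks a new one from shuffled living players via DoOnce, after random delays.
; A looping PlayerCheck timer announces the winner when only one MyPlayer actor is left.
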(event Custom|PlayerCheck
  (bind _outactors (Actor|GetAllActorsOfClass "/Game/PlayerRelated/MyPlayer.MyPlayer_C"))
  (if (== (Utilities|Array|Length _outactors) 1)
    (Utilities|FlowControl|DoOnce false
      (:Completed
        (Utilities|IsValid (Utilities|Array|Get(acopy) _outactors)
          (:Is%20Valid
            (Variables|Default|SetWinningPlayer (Utilities|Array|Get(acopy) _outactors))
            (Development|PrintString (Utilities|String|Append (PlayerState|GetPlayerName (Variables|/Script/Engine.Pawn|GetPlayerState (Utilities|Array|Get(acopy) _outactors))) ": is the winner!") true true "(R=0.072053,G=1.000000,B=0.000000,A=1.000000)" 6.0))
          (:Is%20Not%20Valid
            (Development|PrintString "NEED MORE PLAYERS!" true true "(R=1.000000,G=0.000000,B=0.028391,A=1.000000)")))))))

(event Custom|StartGame
  (if (== (Class|AdvancedSessionsLibrary|GetNumberOfNetworkPlayers) 1)
    (Development|PrintString "NOT ENOUGH PLAYERS!")
    (else
      (CallFunction|RESETGAME)
      (Development|PrintString "STARTING GAME!")
      (Development|PrintString "YOU HAVE 5 SECONDS TO RUN!")
      (Utilities|FlowControl|Delay 5.0)
      (Utilities|Time|SetTimerbyFunctionName 0 "PlayerCheck" 1.0 true :!label _label)
      (bind _outactors (Actor|GetAllActorsOfClass "/Game/PlayerRelated/MyPlayer.MyPlayer_C"))
      (for _array_element _outactors
        (if (Variables|/Game/PlayerRelated/MyPlayer.MyPlayer_C|GetisBomber _array_element)
          (Default|BecomePlayer _array_element false)
          (Development|PrintString "TO PLAYER")
          (goto _label_2 Reset)))
      (bind _outactors_2 (Actor|GetAllActorsOfClass "/Game/PlayerRelated/MyPlayer.MyPlayer_C"))
      (Utilities|Array|Shuffle _outactors_2)
      (for _array_element_2 _outactors_2
        (if (Math|Boolean|ANDBoolean (!= _array_element_2 (Variables|Default|GetWinningPlayer)) (not (Variables|/Game/PlayerRelated/MyPlayer.MyPlayer_C|GetisBomber _array_element_2)) (not (Variables|/Game/PlayerRelated/MyPlayer.MyPlayer_C|GetisDead _array_element_2)))
          (Utilities|FlowControl|DoOnce false :!label _label_2
            (:Completed
              (Default|BecomeBomber _array_element_2 true)
              (Development|PrintString "TO BOMBER")
              (Utilities|FlowControl|Delay (Math|Random|RandomFloatinRange 8.0 15.0))
              (goto _label))))))))

(event Custom|RESET%20GAME
  (Variables|Default|SetWinningPlayer 0)
  (Utilities|FlowControl|DoOnce false) ; enters at Reset
)

(event EventPostLogin
  (params (NewPlayer :type Player%20Controller%20Object%20Reference))
  (bind _playerlist (Variables|Default|GetPlayerList))
  (if (not (Utilities|Array|ContainsItem _playerlist NewPlayer))
    (Utilities|Array|Add _playerlist NewPlayer)))

(event EventOnLogout
  (params (ExitingController :type Controller%20Object%20Reference))
  (for _array_element (Variables|Default|GetPlayerList)
    (if (== _array_element ExitingController)
      (Utilities|Array|RemoveItem (Variables|Default|GetPlayerList) _array_element))))

(fn ConstructionScript)